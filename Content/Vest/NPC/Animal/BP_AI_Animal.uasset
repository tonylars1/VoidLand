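; AI controller for animal NPCs that makes the possessed BPCH_Animal_Master pawn wander at random.
; BeginPlay caches the pawn, then a delayed Tick uses a DoOnce gate to send it to a random reachable point around its current location.
; Arrival calls the pawn's Idle, and either arrival or failure resets the gate after a wait.
; The PlayerSpotted branch starts no movement or other reaction.
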(event Custom|Refresh%20Idle
  (Utilities|FlowControl|DoOnce false) ; enters at Reset
)

(event EventBeginPlay
  (bind _asbpch_animal_master (Utilities|Casting|CastToBPCH_Animal_Master (Pawn|GetControlledPawn)))
  (Variables|Default|SetAnimal%20Pawn _asbpch_animal_master))

(event EventTick
  (params (DeltaSeconds :type Float%20%28single-precision%29))
  (bind _animal_pawn (Variables|Default|GetAnimal%20Pawn))
  (Utilities|FlowControl|Delay 1.0)
  (Utilities|IsValid _animal_pawn
    (:Is%20Valid
      (if (Variables|Default|GetPlayer%20Spotted)
        (Utilities|FlowControl|DoOnce false)
        (else
          (Utilities|FlowControl|DoOnce false
            (:Completed
              (AI|AIMoveTo (Pawn|GetControlledPawn) (.RandomLocation (AI|Navigation|GetRandomReachablePointinRadius (Transformation|GetActorLocation _animal_pawn) 1222.0 0 0)) 0 5e+01 false
                (:OnSuccess
                  (Default|Idle (Variables|Default|GetAnimal%20Pawn))
                  (Utilities|FlowControl|Delay 12.2)
                  (CallFunction|RefreshIdle))
                (:OnFail
                  (Utilities|FlowControl|Delay 2.0)
                  (CallFunction|RefreshIdle))))))))))

(fn ConstructionScript)